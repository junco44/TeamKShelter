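; Basic zombie character for a Left 4 Dead-style game, loading its max health from DT_Zombie by zombie type.
; Only damage instigated by Player-tagged pawns lowers health; at zero, the server ragdolls the body once, stops movement and destroys the actor after a short delay.
; AttackBox overlaps set the AI blackboard's HasOverlapped flag on the server.
; UpdateSpeed exposes max walk speed changes.
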(event OnComponentBeginOverlap(AttackBox)
  (params (OverlappedComponent :type Primitive%20Component%20Object%20Reference) (OtherActor :type Actor%20Object%20Reference) (OtherComp :type Primitive%20Component%20Object%20Reference) (OtherBodyIndex :type Integer) (bFromSweep :type Boolean) (SweepResult :type Hit%20Result%20Structure%20%28by%20ref%29))
  (Networking|SwitchHasAuthority
    (:Authority
      (AI|Components|Blackboard|SetValueasBool (Variables|/Script/AIModule.AIController|GetBlackboard (AI|GetAIController self)) (Variables|Default|GetHasOverlapped) true))))

(event OnComponentEndOverlap(AttackBox)
  (params (OverlappedComponent :type Primitive%20Component%20Object%20Reference) (OtherActor :type Actor%20Object%20Reference) (OtherComp :type Primitive%20Component%20Object%20Reference) (OtherBodyIndex :type Integer))
  (Networking|SwitchHasAuthority
    (:Authority
      (AI|Components|Blackboard|SetValueasBool (Variables|/Script/AIModule.AIController|GetBlackboard (AI|GetAIController self)) (Variables|Default|GetHasOverlapped) false))))

(event Game|Damage|EventAnyDamage
  (params (Damage :type Float%20%28single-precision%29) (DamageType :type Damage%20Type%20Object%20Reference) (InstigatedBy :type Controller%20Object%20Reference) (DamageCauser :type Actor%20Object%20Reference))
  (bind _charactermovement (Variables|Character|GetCharacterMovement))
  (if (Actor|ActorHasTag (Pawn|GetControlledPawn InstigatedBy) "Player")
    (Variables|Default|SetCurHP (- (Variables|Default|GetCurHP) Damage))
    (if (<= (Variables|Default|GetCurHP) 0.0)
      (Networking|SwitchHasAuthority
        (:Authority
          (Utilities|FlowControl|DoOnce false
            (:Completed
              (Physics|SetSimulatePhysics (Variables|Default|GetBody) true)
              (Components|Movement|StopMovementImmediately _charactermovement)
              (Class|NavMovementComponent|StopActiveMovement _charactermovement)
              (Utilities|FlowControl|Delay 1.0)
              (Actor|DestroyActor))))))))

(event EventBeginPlay
  (bind _returnvalue (Utilities|GetDataTableRow "/Game/TEAM_K/Left4Dead/KIM_YoonHan/DT_Zombie.DT_Zombie" (Variables|Default|GetZombie_Type))
    (:then
      (Variables|Default|SetCurHP (.maxhealth _returnvalue)))))

(fn ConstructionScript)

(fn UpdateSpeed
  (params (Speed :type Float%20%28double-precision%29))
  (Variables|/Script/Engine.CharacterMovementComponent|SetMaxWalkSpeed (Variables|Character|GetCharacterMovement) Speed))