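; BP_ItemSpawner is an item spawn point that places a random item at its own transform and respawns one after it is destroyed.
; On BeginPlay only the authority calls DoSpawnItem, which spawns a class picked at random from the SpawnActor list.
; It binds to the spawned item's destroy event dispatcher, and EventItemDestroy sets a five-second timer by function name to run DoSpawnItem again.
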(event EventBeginPlay
  (Networking|SwitchHasAuthority
    (:Authority
      (CallFunction|DoSpawnItem))))

(fn ConstructionScript)

(fn DoSpawnItem
  (bind _returnvalue (Game|SpawnActorfromClass (.OutItem (Utilities|Array|Random (Variables|Default|GetSpawnActor))) (Transformation|GetActorTransform) "Undefined" 0 0))
  (EventDispatchers|BindEventtoEventDispatcherEventDestroy _returnvalue (EventDispatchers|CreateEvent :!event EventItemDestroy)))

(fn EventItemDestroy
  (params (DestroyActor :type Actor%20Object%20Reference))
  (Utilities|Time|SetTimerbyFunctionName 0 "DoSpawnItem" 5.0))