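; BP_DoorTest is an interactable test door that the player can open and close.
; Interact toggles a Status enum and plays or reverses a timeline that drives the Door component's yaw, printing a debug string on each update.
; ShowInfo sets a HUD prompt matching the current state, and ShowOutline toggles custom depth rendering on the door for a focus highlight.
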(event EventBeginPlay)

(event Collision|EventActorBeginOverlap
  (params (OtherActor :type Actor%20Object%20Reference)))

(event EventTick
  (params (DeltaSeconds :type Float%20%28single-precision%29)))

(event EventInteract
  (switch Utilities|FlowControl|Switch|SwitchonEN_DoorStatus (Variables|Default|GetStatus)
    (:NewEnumerator0
      (Variables|Default|SetStatus "NewEnumerator1")
      (bind _doorzrotation (Timeline|Timeline Play)
        (:Update
          (Transformation|SetRelativeRotation (Variables|Default|GetDoor) (Math|Rotator|MakeRotator 0.0 0.0 _doorzrotation) false false)
          (Development|PrintString "Hello"))))
    (:NewEnumerator1
      (Variables|Default|SetStatus "NewEnumerator0")
      (Timeline|Timeline Reverse))))

(event EventShowInfo
  (params (HUD :type Interaction%20Widget%20Object%20Reference))
  (Utilities|IsValid HUD
    (:Is%20Valid
      (switch Utilities|FlowControl|Switch|SwitchonEN_DoorStatus (Variables|Default|GetStatus)
        (:NewEnumerator0
          (Default|SetInfoTest HUD "Press [E] to open door"))
        (:NewEnumerator1
          (Default|SetInfoTest HUD "Press [E] to close door"))))))

(event EventShowOutline
  (params (bIsFocus :type Boolean))
  (Rendering|SetRenderCustomDepth (Variables|Default|GetDoor) bIsFocus))

(fn ConstructionScript)